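; BP_Draw is a card processor in the card game spike that makes the single-player controller draw two cards.
; The Process event casts player controller 0 to PC_SinglePlayer, calls Draw twice, then destroys the actor.
; The Play function repeats the same two draws but ignores its Targets input, leaves the actor alive and returns true.
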(event EventProcess
  (bind _aspc_single_player (Utilities|Casting|CastToPC_SinglePlayer (Game|GetPlayerController 0)))
  (Default|Draw _aspc_single_player)
  (Default|Draw _aspc_single_player)
  (Actor|DestroyActor))

(fn ConstructionScript
  (|CallParentFunction))

(fn Play
  (params (Targets :type Array%20of%20BPI%20Creature%20Interfaces))
  (bind _aspc_single_player (Utilities|Casting|CastToPC_SinglePlayer (Game|GetPlayerController 0)))
  (Default|Draw _aspc_single_player)
  (Default|Draw _aspc_single_player)
  (return true))