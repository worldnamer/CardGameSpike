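; Game mode for a card battle game that runs card play, enemy turns and victory or defeat checks.
; PlayCard spends player energy, gathers targets by the card's targeting type, then spawns the card's class to process itself.
; EndTurn queues enemy AI controllers that act until ActionFinished empties the queue, then resets energy and signals turn end.
; Finishing the victory display advances MAP_01 to MAP_02; random card-reward logic is present but unconnected.
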(event Custom|ActWithNextEnemy
  (if (> (Utilities|Array|Length (Variables|Default|GetEnemiesLeftToAct)) 0)
    (Default|TakeAction (Utilities|Array|Get(acopy) (Variables|Default|GetEnemiesLeftToAct)))
    (else
      (Utilities|FlowControl|Sequence
        (:then_0
          (Class|BPIEnergy|ResetEnergy(Message) (Game|GetPlayerState 0)))
        (:then_1
          ;[1 1 1] This probably should be called StartOfNextTurn, as it has less to do with the end of the turn and more to do with resetting state at the beginning of the turn.
          (Default|CallEndOfTurn))))))

(event EventCheckforVictoryorDefeat
  (bind _returnvalue (Game|Player|GetPlayerPawn 0))
  (bind _outactors (Actor|GetAllActorsOfClass "/Game/CardGameSpike/Core/Characters/P_Enemy.P_Enemy_C"))
  (if (> (Utilities|Array|Length _outactors) 0)
    (Utilities|IsValid _returnvalue
      (:Is%20Valid
        (bind _bisalive (Class|BPICreature|IsAlive(Message) _returnvalue))
        (if (not _bisalive)
          ;[1 1 1] We died, so play defeat animations
          (Default|CallDefeat :!label _label)))
      (:Is%20Not%20Valid
        (goto _label)))
    (else
      ;[1 1 1] No more enemies means we've won
      (Default|CallVictory))))

(event EventEndTurn
  (bind _outactors (Actor|GetAllActorsOfClass "/Game/CardGameSpike/Core/Characters/AIC_Enemy.AIC_Enemy_C"))
  (for _array_element _outactors
    (Utilities|Array|Add (Variables|Default|GetEnemiesLeftToAct) _array_element)
    (CallFunction|ActwithNextEnemy)))

(event EventFinishVictoryDisplay
  (bind _returnvalue (Game|GetCurrentLevelName true))
  (if (Utilities|Enum|Equal(Enum) _returnvalue "MAP_01")
    (Game|OpenLevel(byObjectReference) "/Game/CardGameSpike/Maps/MAP_02.MAP_02")))

(event EventActionFinished
  (params (IndependentActor :type BPI%20Independent%20Actor%20Interface))
  (Utilities|Array|RemoveIndex (Variables|Default|GetEnemiesLeftToAct))
  (CallFunction|ActwithNextEnemy))

(fn ConstructionScript)

(fn PlayCard
  (params (Card :type S%20Card%20Structure) (Target :type P%20Base%20Pawn%20Object%20Reference))
  (bind _successful (Class|BPIEnergy|SpendEnergy(Message) (Game|GetPlayerState 0) (.cost Card)))
  (if _successful
    (switch Utilities|FlowControl|Switch|SwitchonETargets (.targets Card)
      (:NewEnumerator5
        _)
      (:NewEnumerator0
        (bind _asbpi_creature (Utilities|Casting|CastToBPI_Creature (Game|Player|GetPlayerPawn 0)))
        (Utilities|Array|Add (LocalVariables|GetTargets) _asbpi_creature))
      (:NewEnumerator1
        (bind _asbpi_creature_2 (Utilities|Casting|CastToBPI_Creature Target))
        (Utilities|Array|Add (LocalVariables|GetTargets) _asbpi_creature_2))
      (:NewEnumerator2
        (bind _outactors (Actor|GetAllActorsOfClass "/Game/CardGameSpike/Core/Characters/P_Enemy.P_Enemy_C"))
        (for _array_element _outactors
          (bind _asbpi_creature_3 (Utilities|Casting|CastToBPI_Creature _array_element))
          (Utilities|Array|Add (LocalVariables|GetTargets) _asbpi_creature_3))))
    (bind _returnvalue (Game|SpawnActorfromClass (.cardclass Card) (Variables|Default|GetPlaceholderTransform) "AlwaysSpawn" "MultiplyWithRoot" self (LocalVariables|GetTargets) 0))
    (Class|BPICardProcessor|Process(Message) _returnvalue)))