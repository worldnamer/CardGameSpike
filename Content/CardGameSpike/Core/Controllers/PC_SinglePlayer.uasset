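; Single-player PlayerController for a card battler that manages the draw pile, hand and discard, plus the battle UI.
; BeginPlay shuffles the GameInstance deck, binds energy and turn events and draws five cards, reshuffling discards when the pile empties.
; Card drags highlight targets by type; drops line-trace for single targets, then call GM_CardGame's PlayCard and discard.
; It also shows victory, defeat, reward and pause screens.
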(event Custom|UpdateEnergyDisplay
  (params (CurrentEnergy :type Integer) (MaxEnergy :type Integer) (PreviousEnergy :type Integer) (PreviousMaxEnergy :type Integer))
  (Utilities|UpdateEnergyTextWidget CurrentEnergy MaxEnergy))

(event Custom|DrawHand
  (Utilities|FlowControl|Delay 0.2)
  (CallFunction|Draw)
  (Utilities|FlowControl|Delay 0.2)
  (CallFunction|Draw)
  (Utilities|FlowControl|Delay 0.2)
  (CallFunction|Draw)
  (Utilities|FlowControl|Delay 0.2)
  (CallFunction|Draw)
  (Utilities|FlowControl|Delay 0.2)
  (CallFunction|Draw))

(event Custom|UpdateTurnTextWidget
  (params (CurrentTurn :type Integer))
  (Rendering|Components|TextRender|SetText (Variables|/Game/CardGameSpike/UI/Default/WBP_Default.WBP_Default_C|GetT_Turn (Variables|Default|GetW_UI)) (Utilities|Text|ToText(String) (Utilities|String|BuildString(Integer) "Turn " " " CurrentTurn))))

(event EventBeginPlay
  (Utilities|SetUpDrawPile)
  (Utilities|CreateUIWidgets)
  (bind _asps_single_player (Utilities|Casting|CastToPS_SinglePlayer (Game|GetPlayerState 0)))
  (EventDispatchers|BindEventtoEnergyChanged _asps_single_player (EventDispatchers|CreateEvent :!event Custom|UpdateEnergyDisplay))
  (bind _asgs_card_game (Utilities|Casting|CastToGS_CardGame (Game|GetGameState)))
  (EventDispatchers|BindEventtoTurnNumberUpdated _asgs_card_game (EventDispatchers|CreateEvent :!event Custom|UpdateTurnTextWidget))
  (bind _asgm_card_game (Utilities|Casting|CastToGM_CardGame (Game|GetGameMode)))
  (EventDispatchers|BindEventtoEndOfTurn _asgm_card_game (EventDispatchers|CreateEvent :!event DiscardHandandDrawNewOne))
  (CallFunction|DrawHand))

(event EventTogglePauseMenu
  (if (Variables|Default|GetEscapeMenuShowing)
    (Widget|RemovefromParent (Variables|Default|GetW_PauseMenu))
    (Variables|Default|SetEscapeMenuShowing false)
    (else
      (bind _returnvalue (UserInterface|CreateWidget "/Game/CardGameSpike/UI/Menus/WBP_PauseMenu.WBP_PauseMenu_C" self))
      (bind _output_get (Variables|Default|SetW_PauseMenu _returnvalue))
      (UserInterface|Viewport|AddtoViewport _output_get 0)
      (Variables|Default|SetEscapeMenuShowing true))))

(event EventCardDragStart
  (params (WCardBeingDragged :type WBP%20Card%20Object%20Reference) (MousePosition :type Vector%202D%20Structure))
  (bind _w_ui (Variables|Default|GetW_UI))
  (bind _w_targeter (Variables|/Game/CardGameSpike/UI/Default/WBP_Default.WBP_Default_C|GetW_Targeter _w_ui))
  (switch Utilities|FlowControl|Switch|SwitchonETargets (.targets (Variables|/Game/CardGameSpike/UI/Default/WBP_Card.WBP_Card_C|GetCard WCardBeingDragged))
    (:NewEnumerator0
      (bind _outactors (Actor|GetAllActorsOfClass "/Game/CardGameSpike/Characters/Werewolf/P_Werewolf.P_Werewolf_C"))
      (for _array_element _outactors
        (Variables|/Game/CardGameSpike/Core/Characters/P_BasePawn.P_BasePawn_C|SetHighlightState _array_element "NewEnumerator1")
        (bind _returnvalue (Class|WidgetLayoutLibrary|GetViewportWidgetGeometry))
        (Class|Widget|SetRenderTranslation (Variables|/Game/CardGameSpike/UI/Targeter/WBP_Targeter.WBP_Targeter_C|GetP0 _w_targeter) (Class|SlateBlueprintLibrary|ScreentoWidgetLocal _returnvalue (Math|Vector2D|MakeVector2D (/ (.x (Class|SlateBlueprintLibrary|GetAbsoluteSize _returnvalue)) 2.0) (- (.y (Class|SlateBlueprintLibrary|GetAbsoluteSize _returnvalue)) 2e+02)) false))
        (Widget|SetVisibility _w_targeter "Visible")))
    (:NewEnumerator1
      (bind _outactors_2 (Actor|GetAllActorsOfClass "/Game/CardGameSpike/Core/Characters/P_Enemy.P_Enemy_C"))
      (for _array_element_2 _outactors_2
        (Variables|/Game/CardGameSpike/Core/Characters/P_BasePawn.P_BasePawn_C|SetHighlightState _array_element_2 "NewEnumerator1")
        (bind _returnvalue_2 (Class|WidgetLayoutLibrary|GetViewportWidgetGeometry))
        (Class|Widget|SetRenderTranslation (Variables|/Game/CardGameSpike/UI/Targeter/WBP_Targeter.WBP_Targeter_C|GetP0 _w_targeter) (Class|SlateBlueprintLibrary|ScreentoWidgetLocal _returnvalue_2 (Math|Vector2D|MakeVector2D (/ (.x (Class|SlateBlueprintLibrary|GetAbsoluteSize _returnvalue_2)) 2.0) (- (.y (Class|SlateBlueprintLibrary|GetAbsoluteSize _returnvalue_2)) 2e+02)) false))
        (Widget|SetVisibility _w_targeter "Visible")))
    (:NewEnumerator2
      (bind _outactors_3 (Actor|GetAllActorsOfClass "/Game/CardGameSpike/Core/Characters/P_Enemy.P_Enemy_C"))
      (for _array_element_3 _outactors_3
        (Variables|/Game/CardGameSpike/Core/Characters/P_BasePawn.P_BasePawn_C|SetHighlightState _array_element_3 "NewEnumerator3")))))

(event EventCardDragged
  (params (MouseScreenPosition :type Vector%202D%20Structure))
  (bind (_worldposition _worlddirection) (CallFunction|ScreentoWorld MouseScreenPosition))
  (bind _outhit (Collision|LineTraceByChannel _worldposition (+ _worldposition (* _worlddirection 2e+03)) "TraceTypeQuery1" false 0 "None"))
  (Utilities|IsValid (.hitactor _outhit)
    (:Is%20Valid
      (bind _asp_base_pawn (Utilities|Casting|CastToP_BasePawn (.hitactor _outhit))
        (:then
          (Default|Hover _asp_base_pawn))
        (:CastFailed
          (bind _outactors (Actor|GetAllActorsOfClass "/Game/CardGameSpike/Core/Characters/P_BasePawn.P_BasePawn_C"))
          (for _array_element _outactors
            (Default|Unhover _array_element)))))
    (:Is%20Not%20Valid
      _))
  (Default|Reposition (Variables|/Game/CardGameSpike/UI/Default/WBP_Default.WBP_Default_C|GetW_Targeter (Variables|Default|GetW_UI)) (.ViewportPosition (Class|SlateBlueprintLibrary|AbsolutetoViewport MouseScreenPosition))))

(event EventCardDropped
  (params (MouseScreenPosition :type Vector%202D%20Structure) (WCard :type WBP%20Card%20Object%20Reference))
  (bind _card (Variables|/Game/CardGameSpike/UI/Default/WBP_Card.WBP_Card_C|GetCard WCard))
  (switch Utilities|FlowControl|Switch|SwitchonETargets (.targets (Variables|/Game/CardGameSpike/UI/Default/WBP_Card.WBP_Card_C|GetCard WCard))
    (:NewEnumerator5
      ;[1 1 1] No line traces needed, just play the card
      (bind _asgm_card_game (Utilities|Casting|CastToGM_CardGame (Game|GetGameMode)))
      (Default|PlayCard _asgm_card_game _card)
      ;[1 1 1] Update the UI after the card is played
      (bind _index (Default|FindIndexforCard (Variables|/Game/CardGameSpike/UI/Default/WBP_Default.WBP_Default_C|GetW_Hand (Variables|Default|GetW_UI)) WCard :!label _label))
      (Utilities|Array|Insert (Variables|Default|GetDiscard) (Utilities|Array|Get(acopy) (Variables|Default|GetHand) _index))
      (Utilities|Array|RemoveIndex (Variables|Default|GetHand) _index)
      (Default|DiscardCard (Variables|/Game/CardGameSpike/UI/Default/WBP_Default.WBP_Default_C|GetW_Hand (Variables|Default|GetW_UI)) WCard)
      (Utilities|ResetHighlights))
    (:NewEnumerator0
      ;[1 1 1] Check if over player, if so, play card
      (bind _outhit_hitactor (Utilities|ActoratLocation MouseScreenPosition))
      (Utilities|IsValid _outhit_hitactor
        (:Is%20Valid
          (bind _asp_werewolf (Utilities|Casting|CastToP_Werewolf _outhit_hitactor)
            (:then
              (bind _asgm_card_game_2 (Utilities|Casting|CastToGM_CardGame (Game|GetGameMode)))
              (Default|PlayCard _asgm_card_game_2 _card _asp_werewolf)
              (goto _label))
            (:CastFailed
              _)))
        (:Is%20Not%20Valid
          _))
      (Utilities|ResetHighlights :!label _label_2))
    (:NewEnumerator1
      ;[1 1 1] Check if over enemy, if so, play card
      (bind _outhit_hitactor_2 (Utilities|ActoratLocation MouseScreenPosition))
      (Utilities|IsValid _outhit_hitactor_2
        (:Is%20Valid
          (bind _asp_enemy (Utilities|Casting|CastToP_Enemy _outhit_hitactor_2)
            (:then
              (bind _asgm_card_game_3 (Utilities|Casting|CastToGM_CardGame (Game|GetGameMode)))
              (Default|PlayCard _asgm_card_game_3 _card _asp_enemy)
              (goto _label))
            (:CastFailed
              (goto _label_2))))
        (:Is%20Not%20Valid
          (goto _label_2))))
    (:NewEnumerator2
      ;[1 1 1] Play Card against all Enemies
      (bind _asgm_card_game_4 (Utilities|Casting|CastToGM_CardGame (Game|GetGameMode)))
      (Default|PlayCard _asgm_card_game_4 _card)
      (goto _label))))

(event EventShowRewardScreen
  (params (RewardCards :type Array%20of%20S%20Card%20Structures))
  (Variables|/Script/UMG.Widget|SetVisibility (Variables|Default|GetW_UI) "Hidden")
  (bind _returnvalue (UserInterface|CreateWidget "/Game/CardGameSpike/UI/Rewards/WBP_Rewards.WBP_Rewards_C" self))
  (Default|SetRewards _returnvalue RewardCards)
  (UserInterface|Viewport|AddtoViewport _returnvalue 0))

(event EventShowVictoryScreen
  (Widget|SetVisibility (Variables|/Game/CardGameSpike/UI/Default/WBP_Default.WBP_Default_C|GetT_Victory (Variables|Default|GetW_UI)) "Visible")
  (Utilities|Time|SetTimerbyFunctionName 0 "FinishVictoryAnimation" 2.0))

(event EventShowDefeatScreen
  (Widget|SetVisibility (Variables|/Game/CardGameSpike/UI/Default/WBP_Default.WBP_Default_C|GetT_Defeat (Variables|Default|GetW_UI)) "Visible"))

(fn ConstructionScript)

(fn Draw
  (if (> (Utilities|Array|Length (Variables|Default|GetDrawPile)) 0)
    (LocalVariables|SetDrawnCard (Utilities|Array|Get(acopy) (Variables|Default|GetDrawPile)) :!label _label)
    (Utilities|Array|Add (Variables|Default|GetHand) (LocalVariables|GetDrawnCard))
    (Utilities|Array|RemoveIndex (Variables|Default|GetDrawPile))
    (Default|AddCard (Variables|/Game/CardGameSpike/UI/Default/WBP_Default.WBP_Default_C|GetW_Hand (Variables|Default|GetW_UI)) (LocalVariables|GetDrawnCard))
    (else
      (CallFunction|MoveDiscardtoDeck)
      (CallFunction|Shuffle)
      (if (> (Utilities|Array|Length (Variables|Default|GetDrawPile)) 0)
        (goto _label)))))

(fn Shuffle
  (Utilities|Array|Shuffle (Variables|Default|GetDrawPile)))

(fn ScreentoWorld
  (params (MouseScreenPosition :type Vector%202D%20Structure))
  (bind _returnvalue (Class|WidgetLayoutLibrary|GetViewportScale))
  (bind _viewportposition (Class|SlateBlueprintLibrary|AbsolutetoViewport MouseScreenPosition))
  (bind _self self)
  (bind _returnvalue_2 (* _returnvalue _viewportposition))
  (bind (_worldposition _worlddirection) (Class|GameplayStatics|DeprojectScreentoWorld _self _returnvalue_2))
  (return _worldposition _worlddirection))

(fn DiscardHandandDrawNewOne
  (bind _hand (Variables|Default|GetHand))
  (bind _w_ui (Variables|Default|GetW_UI))
  (bind _returnvalue (Utilities|Array|LastIndex _hand))
  (bind _w_hand (Variables|/Game/CardGameSpike/UI/Default/WBP_Default.WBP_Default_C|GetW_Hand _w_ui))
  (bind _cards (Variables|/Game/CardGameSpike/UI/Default/WBP_Hand.WBP_Hand_C|GetCards _w_hand))
  (while (> (Utilities|Array|Length (Variables|Default|GetHand)) 0)
    (Utilities|Array|Add (Variables|Default|GetDiscard) (Utilities|Array|Get(acopy) _hand _returnvalue))
    (Default|DiscardCard _w_hand (Utilities|Array|Get(acopy) _cards (Utilities|Array|LastIndex _cards)))
    (Utilities|Array|RemoveIndex (Variables|Default|GetHand) _returnvalue))
  (CallFunction|DrawHand))

(fn MoveDiscardtoDeck
  (Utilities|Array|AppendArray (Variables|Default|GetDrawPile) (Variables|Default|GetDiscard))
  (Utilities|Array|Clear (Variables|Default|GetDiscard)))

(fn FinishVictoryAnimation
  (Class|BPICardGame|FinishVictoryDisplay(Message) (Game|GetGameMode)))